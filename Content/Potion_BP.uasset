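; Thrown potion projectile that explodes on overlap and knocks punching bags away.
; The construction script sets blast strength and takes launch velocity from the owning character's ThrowVec.
; Static mesh hits briefly scale up the whole actor as a blast before destroying it.
; Bag overlaps apply an always-upward, distance-reduced impulse scaled by the bag's Damage, destroy the potion, print the force and increment Damage, so knockback grows.
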(event OnComponentBeginOverlap(SphereCollision)
  (params (OverlappedComponent :type Primitive%20Component%20Object%20Reference) (OtherActor :type Actor%20Object%20Reference) (OtherComp :type Primitive%20Component%20Object%20Reference) (OtherBodyIndex :type Integer) (bFromSweep :type Boolean) (SweepResult :type Hit%20Result%20Structure%20%28by%20ref%29))
  (Utilities|Casting|CastToStaticMeshActor OtherActor
    (:then
      (Transformation|SetActorScale3D "20.000000,20.000000,20.000000")
      (Utilities|FlowControl|Delay 0.1)
      (Actor|DestroyActor :!label _label))
    (:CastFailed
      ;[1 1 1] This is terrible code and im sorry, but its 12:29 in the morning so I dont care
      (bind _aspunching_bag_blueprint (Utilities|Casting|CastToPunching_Bag_Blueprint OtherActor))
      (Utilities|FlowControl|Sequence
        (:then_0
          (Physics|AddImpulse (Variables|/Script/Engine.Character|GetCapsuleComponent _aspunching_bag_blueprint) (Math|Vector|MakeVector (.X (Math|Vector|BreakVector (* (- (* (Math|Vector|Normalize (- (Transformation|GetActorLocation _aspunching_bag_blueprint) (Transformation|GetActorLocation))) (Variables|Default|GetBlastStrength)) (- (Transformation|GetActorLocation _aspunching_bag_blueprint) (Transformation|GetActorLocation))) (Variables|/Game/Punching_Bag_Blueprint.Punching_Bag_Blueprint_C|GetDamage%25 _aspunching_bag_blueprint)))) (.Y (Math|Vector|BreakVector (* (- (* (Math|Vector|Normalize (- (Transformation|GetActorLocation _aspunching_bag_blueprint) (Transformation|GetActorLocation))) (Variables|Default|GetBlastStrength)) (- (Transformation|GetActorLocation _aspunching_bag_blueprint) (Transformation|GetActorLocation))) (Variables|/Game/Punching_Bag_Blueprint.Punching_Bag_Blueprint_C|GetDamage%25 _aspunching_bag_blueprint)))) (Math|Float|Absolute(Float) (.Z (Math|Vector|BreakVector (* (- (* (Math|Vector|Normalize (- (Transformation|GetActorLocation _aspunching_bag_blueprint) (Transformation|GetActorLocation))) (Variables|Default|GetBlastStrength)) (- (Transformation|GetActorLocation _aspunching_bag_blueprint) (Transformation|GetActorLocation))) (Variables|/Game/Punching_Bag_Blueprint.Punching_Bag_Blueprint_C|GetDamage%25 _aspunching_bag_blueprint)))))) "None" true)
          (goto _label))
        (:then_1
          (Development|PrintString (Utilities|String|ToString(Float) (Math|Vector|VectorLength (Math|Vector|MakeVector (.X (Math|Vector|BreakVector (* (- (* (Math|Vector|Normalize (- (Transformation|GetActorLocation _aspunching_bag_blueprint) (Transformation|GetActorLocation))) (Variables|Default|GetBlastStrength)) (- (Transformation|GetActorLocation _aspunching_bag_blueprint) (Transformation|GetActorLocation))) (Variables|/Game/Punching_Bag_Blueprint.Punching_Bag_Blueprint_C|GetDamage%25 _aspunching_bag_blueprint)))) (.Y (Math|Vector|BreakVector (* (- (* (Math|Vector|Normalize (- (Transformation|GetActorLocation _aspunching_bag_blueprint) (Transformation|GetActorLocation))) (Variables|Default|GetBlastStrength)) (- (Transformation|GetActorLocation _aspunching_bag_blueprint) (Transformation|GetActorLocation))) (Variables|/Game/Punching_Bag_Blueprint.Punching_Bag_Blueprint_C|GetDamage%25 _aspunching_bag_blueprint)))) (Math|Float|Absolute(Float) (.Z (Math|Vector|BreakVector (* (- (* (Math|Vector|Normalize (- (Transformation|GetActorLocation _aspunching_bag_blueprint) (Transformation|GetActorLocation))) (Variables|Default|GetBlastStrength)) (- (Transformation|GetActorLocation _aspunching_bag_blueprint) (Transformation|GetActorLocation))) (Variables|/Game/Punching_Bag_Blueprint.Punching_Bag_Blueprint_C|GetDamage%25 _aspunching_bag_blueprint))))))))))
        (:then_2
          (Variables|/Game/Punching_Bag_Blueprint.Punching_Bag_Blueprint_C|SetDamage%25 _aspunching_bag_blueprint (+ (Variables|/Game/Punching_Bag_Blueprint.Punching_Bag_Blueprint_C|GetDamage%25 _aspunching_bag_blueprint) 0.05)))))))

(event EventBeginPlay)

(event EventTick
  (params (DeltaSeconds :type Float%20%28single-precision%29)))

(fn ConstructionScript
  (Utilities|FlowControl|Sequence
    (:then_0
      (Variables|Default|SetBlastStrength 5e+02))
    (:then_1
      (bind _ascharacter_blueprint (Utilities|Casting|CastToCharacter_Blueprint (Components|GetOwner)))
      (Game|Components|ProjectileMovement|SetVelocityinLocalSpace (Variables|Default|GetProjectileMovement) (Variables|/Game/Character_Blueprint.Character_Blueprint_C|GetThrowVec _ascharacter_blueprint)))))