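; VortexPlunge_BP is a fall-out hazard that costs any overlapping Wizard_BP a life and plays an audio component on it.
; With lives left, the wizard's velocity is zeroed, Damage is reset to 0.4 and it moves to a fixed respawn point.
; At -1 lives it leaves FinalGamemode's PlayersArray; when one player remains, a Winner widget and sound precede opening TestMap after a delay.
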(event EventBeginPlay)

(event Collision|EventActorBeginOverlap
  (params (OtherActor :type Actor%20Object%20Reference))
  (bind _aswizard_bp (Utilities|Casting|CastToWizard_BP OtherActor))
  (bind _returnvalue (AddComponent|AddAudioComponent _aswizard_bp false))
  (Audio|Components|Audio|Play _returnvalue 0.0)
  (bind _result (Math|Integer|DecrementInt (Variables|/Game/Final/Blueprints/Wizard_BP.Wizard_BP_C|GetLives _aswizard_bp))
    (:%20%20
      (Math|Integer|CompareInt _result -1
        (:>
          (Variables|/Script/Engine.MovementComponent|SetVelocity (Variables|/Script/Engine.Character|GetCharacterMovement _aswizard_bp) "0, 0, 0")
          (Variables|/Game/Final/Blueprints/Wizard_BP.Wizard_BP_C|Setdamage _aswizard_bp 0.4)
          (Transformation|SetRelativeLocation (Variables|/Script/Engine.Actor|GetRootComponent _aswizard_bp) "0.000000,-50.000000,192.000000" false false))
        (:==
          (bind _asfinal_gamemode (Utilities|Casting|CastToFinalGamemode (Game|GetGameMode)))
          (for (_array_element _array_index) (Variables|/Game/Final/Blueprints/FinalGamemode.FinalGamemode_C|GetplayersArray _asfinal_gamemode)
            (if (== _aswizard_bp _array_element)
              (Utilities|Array|RemoveIndex (Variables|/Game/Final/Blueprints/FinalGamemode.FinalGamemode_C|GetplayersArray _asfinal_gamemode) _array_index)))
          (Math|Integer|CompareInt (Utilities|Array|Length (Variables|/Game/Final/Blueprints/FinalGamemode.FinalGamemode_C|GetplayersArray _asfinal_gamemode)) 1
            (:==
              (bind _returnvalue_2 (UserInterface|CreateWidget "/Game/Final/Widgets/Winner.Winner_C" (Game|GetPlayerController 0)))
              (UserInterface|Viewport|AddtoViewport _returnvalue_2 0)
              (Audio|PlaySound2D "/Game/Final/Sound/Menu_sounds/quick_dramatic_sound_cue.quick_dramatic_sound_cue" 5.0 1.0 0.0 0 0)
              (Utilities|FlowControl|Delay 2.0)
              (Game|OpenLevel(byName) "TestMap"))))))))

(event EventTick
  (params (DeltaSeconds :type Float%20%28single-precision%29)))

(fn ConstructionScript)