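; Player wizard character for a multiplayer potion brawler, with twin-stick movement and aiming, charged potion throws, a potion-fueled bomb jump and a cooldown dash that shoves characters.
; Holding Throw builds a charge that scales the throw vector and arrow material; potions regenerate while grounded, and special potions add freeze, cluster or drinkable golden-skin effects.
; Hits launch the wizard in proportion to accumulated Damage, which also drives smoke particles and cloak and hat tint.
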(event OnComponentHit(CapsuleComponent)
  (params (HitComponent :type Primitive%20Component%20Object%20Reference) (OtherActor :type Actor%20Object%20Reference) (OtherComp :type Primitive%20Component%20Object%20Reference) (NormalImpulse :type Vector :default "0, 0, 0") (Hit :type Hit%20Result%20Structure%20%28by%20ref%29))
  ;[1 1 1] Dash push
  (if (Variables|Dashing|Getdashing)
    (bind _ascharacter (Utilities|Casting|CastToCharacter OtherActor))
    (Character|LaunchCharacter _ascharacter (- (Variables|Dashing|GetdashEnd) (Variables|Dashing|GetdashStart)) false false)))

(event Custom|Haptic%20effect
  ;[1 1 1] Controller rumble
  (Game|Feedback|PlayDynamicForceFeedback (Game|GetPlayerController (Variables|Default|GetplayerControllerIndex)) 1.0 0.5 true true true true))

(event Custom|damageUpdated
  (bind _starting_damage (Variables|Default|GetStarting%20Damage))
  (bind _damage (Variables|Default|Getdamage))
  (bind _returnvalue (- _damage _starting_damage))
  (bind _returnvalue_2 (Math|Float|MapRangeClamped _returnvalue 0.0 3.0 0.0 1.0))
  ;[1 1 1] Damage update
  (Effects|Components|ParticleSystem|SetFloatParameter (Variables|Default|GetWizard_Hit_Effects) "ParticleRate" _returnvalue)
  (Rendering|Material|SetScalarParameterValue (Variables|Default|GetCloakColor) "Damage_Lerp" _returnvalue_2 :!class /Script/Engine.MaterialInstanceDynamic)
  (Rendering|Material|SetScalarParameterValue (Variables|Default|GetHatColor) "Damage_Lerp" _returnvalue_2 :!class /Script/Engine.MaterialInstanceDynamic))

(event Custom|Play_Hit_Animation
  ;[1 1 1] Because You can't play a montage in a function
  (Animation|Montage|PlayMontage (Variables|Character|GetMesh) "/Game/Final/Animation/Montages/HitReact_Montage.HitReact_Montage"))

(event Custom|applyStatusEffect
  (bind _charactermovement (Variables|Character|GetCharacterMovement))
  ;[1 1 1] Apply status effect
  (switch Utilities|FlowControl|Switch|SwitchonSTATUS_EFFECTS (Variables|SpecialPotions|GetstatusEffect)
    (:NewEnumerator0
      (Variables|/Script/Engine.CharacterMovementComponent|SetMaxWalkSpeed _charactermovement 5e+01)
      (Utilities|FlowControl|Delay 5.0)
      (Variables|/Script/Engine.CharacterMovementComponent|SetMaxWalkSpeed _charactermovement 1.5e+02))
    (:NewEnumerator1
      (Variables|Default|SetforceMultiplier 0.5)
      (Variables|Default|SetdamageMultiplier 0.0001)
      (Utilities|FlowControl|Delay 1e+01)
      (Variables|Default|SetforceMultiplier 1.0)
      (Variables|Default|SetdamageMultiplier 0.0002))))

(event EventBeginPlay
  (bind _cloakcolor (Variables|Default|GetCloakColor))
  (bind _potion (Variables|Default|GetPotion))
  ;[1 1 1] Set Wizard materials
  (Variables|Default|Setdamage (Variables|Default|GetStarting%20Damage))
  (Utilities|FlowControl|Delay 0.1)
  (bind _returnvalue (Rendering|Material|GetVectorParameterValue _cloakcolor "PotionPrimary" :!class /Script/Engine.MaterialInstanceDynamic))
  (bind _returnvalue_2 (Rendering|Material|GetVectorParameterValue _cloakcolor "PotionSecondary" :!class /Script/Engine.MaterialInstanceDynamic))
  (bind _returnvalue_3 (Rendering|Material|CreateDynamicMaterialInstance _potion 1 "/Game/Final/Materials/Liquids/Master_Liquid_M.Master_Liquid_M" "None" :!class /Script/Engine.PrimitiveComponent))
  (Rendering|Material|SetMaterial _potion 1 _returnvalue_3)
  (Rendering|Material|SetVectorParameterValue _returnvalue_3 "PotionPrimary" _returnvalue :!class /Script/Engine.MaterialInstanceDynamic)
  (Rendering|Material|SetVectorParameterValue _returnvalue_3 "PotionSecondary" _returnvalue_2 :!class /Script/Engine.MaterialInstanceDynamic))

(event Collision|EventActorBeginOverlap
  (params (OtherActor :type Actor%20Object%20Reference)))

(event EventTick
  (params (DeltaSeconds :type Float%20%28single-precision%29))
  (bind _returnvalue (Transformation|GetVelocity))
  (bind _throwcharge (Variables|Throwing|GetthrowCharge))
  (bind _numpotions (Variables|Potions|GetnumPotions))
  (bind (_x _y _z) (Math|Vector|BreakVector _returnvalue))
  (Utilities|FlowControl|Sequence
    (:then_0
      ;[1 1 1] Clamp downward acceleration
      (Variables|/Script/Engine.MovementComponent|SetVelocity (Variables|Character|GetCharacterMovement) (Math|Vector|MakeVector _x _y (Math|Float|Clamp(Float) _z (Variables|Default|GetmaxFallVelocity) 1e+08))))
    (:then_1
      ;[1 1 1] Check potion increment
      (if (and (< _numpotions (Variables|Potions|GetmaxPotions)) (not (AI|Components|NavMovement|IsFalling (Variables|Character|GetCharacterMovement))))
        (Utilities|FlowControl|DoOnce false :!label _label
          (:Completed
            (Utilities|FlowControl|Delay (Variables|Potions|GetpotionDelay))
            (Math|Integer|IncrementInt _numpotions
              (:%20%20
                (goto _label Reset)))))))
    (:then_2
      ;[1 1 1] Charge throw
      (if (Variables|Throwing|GetthrowHeld)
        (Math|Float|IncrementFloat _throwcharge
          (:%20%20
            (Rendering|Material|SetScalarParameterValue (Variables|Default|GetThrowArrowMat) "Charge" (Math|Float|Clamp(Float) (/ _throwcharge (Variables|Throwing|GetmaxCharge))) :!class /Script/Engine.MaterialInstanceDynamic)))))))

(event Input|ActionEvents|InputActionReset
  (params (Key :type Key%20Structure))
  ;[1 1 1] Reset
  (:Pressed
    (if (== (Variables|Default|GetplayerControllerIndex self) 0)
      (Development|ExecuteConsoleCommand "RestartLevel" 0))))

(event Input|ActionEvents|InputActionDash
  (params (Key :type Key%20Structure))
  ;[1 1 1] Dash Ability
  (:Pressed
    (Utilities|FlowControl|DoOnce false :!label _label
      (:Completed
        (Variables|Dashing|SetcanDash false)
        (Variables|Dashing|Setdashing true)
        (Animation|Montage|PlayMontage (Variables|Character|GetMesh) "/Game/Final/Animation/Montages/Dash_Montage.Dash_Montage"
          (:then
            (CallFunction|SetDashStartEnd (Transformation|GetActorLocation) (Class|Pawn|GetLastMovementInputVector))
            (Audio|PlaySoundatLocation "/Game/Final/Sound/Gameplay_sounds/dashing_whoosh.dashing_whoosh" (Transformation|GetWorldLocation (Variables|Collision|GetCapsuleComponent)) "0, 0, 0" 1.0 1.0 0.0 0 0 0)
            (bind _dashalpha (Timeline|Dash PlayFromStart)
              (:Update
                (Transformation|SetWorldLocation (Variables|Collision|GetCapsuleComponent) (Math|Vector|Lerp(Vector) (Variables|Dashing|GetdashStart) (Variables|Dashing|GetdashEnd) _dashalpha) true false))
              (:Finished
                (Variables|Dashing|Setdashing false)
                (Utilities|FlowControl|Delay (Variables|Dashing|GetdashCooldown)) ; Duration is the cooldown
                (Variables|Dashing|SetcanDash true)
                (goto _label Reset)))))))))

(event Input|ActionEvents|InputActionThrow
  (params (Key :type Key%20Structure))
  (bind _facevec (Variables|Default|GetfaceVec))
  ;[1 1 1] Throw
  (:Pressed
    (if (and (> (Variables|SpecialPotions|GetnumSpecialPotions) 0) (Utilities|Enum|Equal(Enum) (Variables|SpecialPotions|GetspecialPotion) "NewEnumerator2"))
      (CallFunction|DrinkPotion)
      (elif (> (Variables|Potions|GetnumPotions) 0) ; If we have potions to throw
        (Variables|Throwing|SetthrowHeld true)
        (Variables|Throwing|SetthrowCharge 0.0)
        (Rendering|SetVisibility (Variables|Default|GetPotion) true false)
        (if (Variables|Throwing|GetcanThrow)
          (Animation|Montage|PlayMontage (Variables|Character|GetMesh) "/Game/Final/Animation/Montages/ThrowWithCharge_Montage.ThrowWithCharge_Montage"
            (:OnInterrupted
              (Variables|Throwing|SetcanThrow true))))
        (else
          (Utilities|FlowControl|DoOnce false :!label _label
            (:Completed
              (Animation|Montage|PlayMontage (Variables|Character|GetMesh) "/Game/Final/Animation/Montages/Shrug_Montage.Shrug_Montage"
                (:OnCompleted
                  (goto _label Reset))
                (:OnBlendOut
                  (goto _label Reset))
                (:OnInterrupted
                  (goto _label Reset)))))))))
  (:Released
    (Variables|Throwing|SetthrowHeld false)
    (if (and (== (stale Input|AxisEvents|InputAxisRightThrowAxis AxisValue) 0.0) (== (stale Input|AxisEvents|InputAxisUpThrowAxis AxisValue) 0.0))
      (CallFunction|SetThrowArrowCharge (.y _facevec) (.x _facevec)) ; if we aren't aiming just throw where we are facing
    )
    (Variables|Throwing|SetcurrentThrowVector (Variables|Throwing|GetmutableThrowVector))
    (Rendering|SetVisibility (Variables|Default|GetPotion) false false)))

(event Input|ActionEvents|InputActionJump
  (params (Key :type Key%20Structure))
  ;[1 1 1] Jumping
  (:Pressed
    (if (> (Variables|Potions|GetnumPotions) 0) ; If we have potions to throw
      (Animation|Montage|PlayMontage (Variables|Character|GetMesh) "/Game/Final/Animation/Montages/PotionJump_Montage.PotionJump_Montage"
        (:then
          (CallFunction|ExplosionSound)
          (CallFunction|BombJump)
          (CallFunction|HapticEffect))))))

(event Input|AxisEvents|InputAxisRightThrowAxis
  (params (AxisValue :type Float%20%28single-precision%29))
  ;[1 1 1] Set throw arrow
  (Utilities|FlowControl|Sequence
    (:then_0
      (CallFunction|SetThrowArrowCharge AxisValue (stale Input|AxisEvents|InputAxisUpThrowAxis AxisValue)))
    (:then_1
      ;[1 1 1] Rotate Character
      (if (> (Math|Vector|VectorLength (Math|Vector|MakeVector (stale Input|AxisEvents|InputAxisUpThrowAxis AxisValue) AxisValue 0.0)) 0.5)
        (Variables|Default|SetfaceVec (Math|Vector|MakeVector (stale Input|AxisEvents|InputAxisUpThrowAxis AxisValue) AxisValue 0.0))
        (Pawn|SetControlRotation (Pawn|GetController) (Math|Conversions|RotationFromXVector (Math|Vector|MakeVector (stale Input|AxisEvents|InputAxisUpThrowAxis AxisValue) AxisValue 0.0)))))))

(event Input|AxisEvents|InputAxisUpThrowAxis
  (params (AxisValue :type Float%20%28single-precision%29))
  ;[1 1 1] Set throw arrow
  (Utilities|FlowControl|Sequence
    (:then_0
      (CallFunction|SetThrowArrowCharge (stale Input|AxisEvents|InputAxisRightThrowAxis AxisValue) AxisValue))
    (:then_1
      ;[1 1 1] Rotate Character
      (if (> (Math|Vector|VectorLength (Math|Vector|MakeVector AxisValue (stale Input|AxisEvents|InputAxisRightThrowAxis AxisValue) 0.0)) 0.5)
        (Variables|Default|SetfaceVec (Math|Vector|MakeVector AxisValue (stale Input|AxisEvents|InputAxisRightThrowAxis AxisValue) 0.0))
        (Pawn|SetControlRotation (Pawn|GetController) (Math|Conversions|RotationFromXVector (Math|Vector|MakeVector AxisValue (stale Input|AxisEvents|InputAxisRightThrowAxis AxisValue) 0.0)))))))

(event Input|AxisEvents|InputAxisUpMoveAxis
  (params (AxisValue :type Float%20%28single-precision%29))
  ;[1 1 1] Movement
  (Pawn|Input|AddMovementInput (Math|Vector|MakeVector AxisValue 0.0 0.0) 1.0 false))

(event Input|AxisEvents|InputAxisRightMoveAxis
  (params (AxisValue :type Float%20%28single-precision%29))
  ;[1 1 1] Movement
  (Pawn|Input|AddMovementInput (Math|Vector|MakeVector 0.0 AxisValue 0.0) 1.0 false))

(fn ConstructionScript
  (bind _returnvalue (Rendering|Material|CreateDynamicMaterialInstance (Variables|Default|GetThrowArrow) 0 "/Game/Final/Materials/ThrowArrow_M.ThrowArrow_M" "None" :!class /Script/Engine.PrimitiveComponent))
  (Variables|Default|SetThrowArrowMat _returnvalue))

(fn ApplyBombImpulse
  (params (NewParam :type Vector))
  (bind _output_get (LocalVariables|SetbombImpulse NewParam))
  (CallFunction|PlayHitAnimation)
  (Character|LaunchCharacter (* (Math|Vector|MakeVector (.X (Math|Vector|BreakVector (* _output_get (Variables|Default|Getdamage)))) (.Y (Math|Vector|BreakVector (* _output_get (Variables|Default|Getdamage)))) (Math|Float|Absolute(Float) (.Z (Math|Vector|BreakVector (* _output_get (Variables|Default|Getdamage)))))) (Variables|Default|GetforceMultiplier)) false false)
  (Variables|Default|Setdamage (+ (Variables|Default|Getdamage) (* (Math|Vector|VectorLength _output_get) (Variables|Default|GetdamageMultiplier))))
  (CallFunction|DamageUpdated)
  (CallFunction|HapticEffect))

(fn ThrowBomb
  (bind _mesh (Variables|Character|GetMesh))
  (bind _returnvalue (Transformation|GetSocketLocation _mesh "Potion"))
  (bind _returnvalue_2 (Math|Transform|MakeTransform _returnvalue))
  (if (> (Variables|SpecialPotions|GetnumSpecialPotions) 0)
    (switch Utilities|FlowControl|Switch|SwitchonSPECIAL_POTIONS (Variables|SpecialPotions|GetspecialPotion)
      (:NewEnumerator0
        (Game|SpawnActorfromClass "/Game/Final/Blueprints/SpecialPotions/FreezePotion_BP.FreezePotion_BP_C" _returnvalue_2 "AlwaysSpawn" self 0))
      (:NewEnumerator1
        (Game|SpawnActorfromClass "/Game/Final/Blueprints/SpecialPotions/ClusterPotion_BP.ClusterPotion_BP_C" _returnvalue_2 "AlwaysSpawn" self 0)))
    (bind _result (Math|Integer|DecrementInt (Variables|SpecialPotions|GetnumSpecialPotions))
      (:%20%20
        (Variables|Throwing|SetthrowCharge 0.0)
        (if (not (> _result 0))
          (Variables|SpecialPotions|SetspecialPotion "NewEnumerator3"))))
    (else
      (bind _returnvalue_3 (Game|SpawnActorfromClass "/Game/Final/Blueprints/Potion_BP.Potion_BP_C" _returnvalue_2 "AlwaysSpawn" self 0))
      (if (Utilities|IsValid _returnvalue_3)
        (bind _returnvalue_4 (Rendering|Material|GetVectorParameterValue (Variables|Default|GetCloakColor) "Cloak" :!class /Script/Engine.MaterialInstanceDynamic))
        (Variables|/Game/Final/Blueprints/Potion_BP.Potion_BP_C|SetExplosionColor _returnvalue_3 _returnvalue_4)
        (bind _returnvalue_5 (Rendering|Material|GetVectorParameterValue (Variables|Default|GetCloakColor) "Cloak" :!class /Script/Engine.MaterialInstanceDynamic))
        (Default|SetPotColour _returnvalue_3 (.r _returnvalue_5) (.g _returnvalue_5) (.b _returnvalue_5)))
      (Math|Integer|DecrementInt (Variables|Potions|GetnumPotions)
        (:%20%20
          (Variables|Throwing|SetthrowCharge 0.0)
          (Rendering|Material|SetScalarParameterValue (Variables|Default|GetThrowArrowMat) "Charge" 0.0 :!class /Script/Engine.MaterialInstanceDynamic)
          (bind _returnvalue_6 (Rendering|Material|CreateDynamicMaterialInstance "/Game/Final/Materials/Liquids/Master_Liquid_M.Master_Liquid_M" "None" :!class /Script/Engine.KismetMaterialLibrary))
          (if (Utilities|IsValid (Variables|/Game/Final/Blueprints/Potion_BP.Potion_BP_C|GetPotionBottle _returnvalue_3))
            (Rendering|Material|SetMaterial (Variables|/Game/Final/Blueprints/Potion_BP.Potion_BP_C|GetPotionBottle _returnvalue_3) 1 _returnvalue_6)
            (Utilities|FlowControl|Sequence
              (:then_0
                (bind _returnvalue_7 (Rendering|Material|GetVectorParameterValue (Variables|Default|GetCloakColor) "PotionPrimary" :!class /Script/Engine.MaterialInstanceDynamic))
                (Rendering|Material|SetVectorParameterValue _returnvalue_6 "PotionPrimary" _returnvalue_7 :!class /Script/Engine.MaterialInstanceDynamic))
              (:then_1
                (bind _returnvalue_8 (Rendering|Material|GetVectorParameterValue (Variables|Default|GetCloakColor) "PotionSecondary" :!class /Script/Engine.MaterialInstanceDynamic))
                (Rendering|Material|SetVectorParameterValue _returnvalue_6 "PotionSecondary" _returnvalue_8 :!class /Script/Engine.MaterialInstanceDynamic)))))))))

(fn BombJump
  (Character|LaunchCharacter (+ (Variables|Jumping|GetbombJumpVector) (* (Variables|Jumping|GetchargeJumpImpulse) (Math|Float|Clamp(Float) (/ (Variables|Throwing|GetthrowCharge) (Variables|Throwing|GetmaxCharge))))) false true)
  (CallFunction|PotionBreakSound)
  (CallFunction|PlayHitSounds)
  (Effects|SpawnEmitteratLocation "/Game/Final/Particles/Explosion/Explosion_P.Explosion_P" (Transformation|GetActorLocation))
  (CallFunction|BombJumpAOE)
  (Math|Integer|DecrementInt (Variables|Potions|GetnumPotions)
    (:%20%20
      (Variables|Default|Setdamage (+ (Variables|Default|Getdamage) (LocalVariables|GetbombJumpDamage)))
      (CallFunction|DamageUpdated)
      (Variables|Throwing|SetthrowCharge 0.0)
      (Rendering|Material|SetScalarParameterValue (Variables|Default|GetThrowArrowMat) "Charge" 0.0 :!class /Script/Engine.MaterialInstanceDynamic))))

(fn SetDashStartEnd
  (params (startLocation :type Vector) (lastMovementVec :type Vector))
  (bind _output_get (Variables|Dashing|SetdashStart startLocation))
  (Variables|Dashing|SetdashEnd (+ _output_get (* (Math|Vector|Normalize lastMovementVec) (Variables|Dashing|GetdashDistance)))))

(fn AxisFunction
  (params (inx :type Float%20%28single-precision%29) (iny :type Float%20%28single-precision%29))
  (bind _returnvalue (Math|Vector|MakeVector inx iny 0.0))
  (bind _returnvalue_2 (Math|Vector|Normalize _returnvalue))
  (bind (_x _y) (Math|Vector|BreakVector _returnvalue_2))
  (return _x _y))

(fn SetThrowArrowCharge
  (params (rightAxis :type Float%20%28single-precision%29) (upAxis :type Float%20%28single-precision%29))
  (bind _returnvalue (Transformation|GetVelocity))
  (bind _throwcharge (Variables|Throwing|GetthrowCharge))
  (bind _maxcharge (Variables|Throwing|GetmaxCharge))
  (bind _chargerate (Variables|Throwing|GetchargeRate))
  (bind (_x _y) (Math|Vector|BreakVector _returnvalue))
  (bind _returnvalue_2 (* _throwcharge _chargerate))
  (bind _returnvalue_3 (/ _returnvalue_2 _maxcharge))
  (bind _returnvalue_4 (Math|Float|Clamp(Float) _returnvalue_3))
  (bind _returnvalue_5 (/ _returnvalue_4 4.0))
  (bind _returnvalue_6 (Math|Vector|MakeVector upAxis rightAxis _returnvalue_5))
  (bind _returnvalue_7 (Math|Vector|Normalize _returnvalue_6))
  ;[1 1 1] Charge shot
  (Utilities|FlowControl|Sequence
    (:then_0
      (bind _output_get (Variables|Throwing|SetmutableThrowVector (+ (* (Math|Vector|Lerp(Vector) (* _returnvalue_7 (LocalVariables|GetminThrow)) (* _returnvalue_7 (LocalVariables|GetmaxThrow)) (Math|Float|Clamp(Float) (/ (* (Variables|Throwing|GetthrowCharge) (Variables|Throwing|GetchargeRate)) (Variables|Throwing|GetmaxCharge)))) (Variables|Throwing|GetthrowStrength)) (* (Math|Vector|MakeVector _x _y 0.0) (Variables|Throwing|GetvelocityInfluence))))))
    (:then_1
      (Variables|Throwing|SetstickRadius _returnvalue_4))))

(fn ExplosionSound
  (bind _returnvalue (Math|Random|RandomFloatinRange 0.5 1.5))
  (bind _capsulecomponent (Variables|Collision|GetCapsuleComponent))
  (bind _returnvalue_2 (Transformation|GetWorldLocation _capsulecomponent))
  (switch int (Math|Random|RandomInteger 3)
    (:0
      (Audio|PlaySoundatLocation "/Game/Final/Sound/Gameplay_sounds/explosion_1.explosion_1" _returnvalue_2 "0, 0, 0" 1.0 _returnvalue 0.15 0 0 0))
    (:1
      (Audio|PlaySoundatLocation "/Game/Final/Sound/Gameplay_sounds/explosion_2.explosion_2" _returnvalue_2 "0, 0, 0" 1.5 _returnvalue 0.0 0 0 0))
    (:2
      (Audio|PlaySoundatLocation "/Game/Final/Sound/Gameplay_sounds/explosion_3.explosion_3" _returnvalue_2 "0, 0, 0" 1.7 _returnvalue 0.0 0 0 0))))

(fn PotionBreakSound
  (bind _capsulecomponent (Variables|Collision|GetCapsuleComponent))
  (bind _returnvalue (Transformation|GetWorldLocation _capsulecomponent))
  (switch int (Math|Random|RandomInteger 2)
    (:0
      (Audio|PlaySoundatLocation "/Game/Final/Sound/Gameplay_sounds/potion_break_3.potion_break_3" _returnvalue "0, 0, 0" 1.0 1.0 0.0 0 0 0))
    (:1
      (Audio|PlaySoundatLocation "/Game/Final/Sound/Gameplay_sounds/potion_break_4.potion_break_4" _returnvalue "0, 0, 0" 1.0 1.0 0.0 0 0 0))))

(fn DamageSmoldering
  (bind _returnvalue (Effects|SpawnEmitterAttached (Variables|/Script/Engine.ParticleSystemComponent|GetTemplate (Variables|Default|GetWizard_Hit_Effects)) (Variables|Character|GetMesh) "None" "0, 0,900.000000" "0, 0, 0" "1.000000,1.000000,1.000000" "SnapToTarget"))
  (Effects|Components|ParticleSystem|SetFloatParameter _returnvalue "Rate" 1.0))

(fn BombJumpAOE
  (bind _asfinal_gamemode (Utilities|Casting|CastToFinalGamemode (Game|GetGameMode)))
  (for _array_element (Variables|/Game/Final/Blueprints/FinalGamemode.FinalGamemode_C|GetplayersArray _asfinal_gamemode)
    (if (and (!= _array_element self) (< (Math|Vector|VectorLength (- (Transformation|GetWorldLocation (Variables|/Script/Engine.Character|GetCapsuleComponent _array_element)) (- (Transformation|GetWorldLocation (Variables|Collision|GetCapsuleComponent)) "0, 0,10.000000"))) (Variables|Jumping|GetbombJumpAOERadius)))
      (CallFunction|ApplyBombImpulse _array_element (- (* (Math|Vector|Normalize (- (Transformation|GetWorldLocation (Variables|/Script/Engine.Character|GetCapsuleComponent _array_element)) (- (Transformation|GetWorldLocation (Variables|Collision|GetCapsuleComponent)) "0, 0,10.000000"))) (Variables|Jumping|GetbombJumpDamageMultiplier)) (- (Transformation|GetWorldLocation (Variables|/Script/Engine.Character|GetCapsuleComponent _array_element)) (- (Transformation|GetWorldLocation (Variables|Collision|GetCapsuleComponent)) "0, 0,10.000000")))))))

(fn SetWizColour
  (params (Number :type Integer))
  (switch int Number
    (:0
      (Variables|Default|SetWizard_Colour "0.010000,0.000000,0.800000"))
    (:1
      (Variables|Default|SetWizard_Colour "0.000000,0.600000,0.000000"))
    (:2
      (Variables|Default|SetWizard_Colour "0.600000,0.000000,0.000000"))
    (:3
      (Variables|Default|SetWizard_Colour "9.000000,0.100000,0.800000"))))

(fn DrinkPotion
  (Rendering|SetVisibility (Variables|Default|GetPotion) true false)
  (Animation|PlayAnimMontage "/Game/Final/Animation/Montages/Drink_Montage.Drink_Montage" 1.0 "None")
  (Variables|SpecialPotions|SetstatusEffect "NewEnumerator1")
  (bind _result (Math|Integer|DecrementInt (Variables|SpecialPotions|GetnumSpecialPotions))
    (:%20%20
      (Variables|Throwing|SetthrowCharge 0.0)
      (if (> _result 0)
        _
        (else
          (Variables|SpecialPotions|SetspecialPotion "NewEnumerator3")))
      (CallFunction|ApplyStatusEffect))))

(fn PlayHitSounds
  (bind _returnvalue (Math|Random|RandomFloatinRange 0.9 1.1))
  (bind _mesh (Variables|Character|GetMesh))
  (bind _returnvalue_2 (Transformation|GetWorldLocation _mesh))
  ;[1 1 1] Randomized grunt noise is played when hit.
  (switch int (Math|Random|RandomInteger 5)
    (:0
      (Audio|PlaySoundatLocation "/Game/Final/Sound/Character_sounds/grunt_5.grunt_5" _returnvalue_2 "0, 0, 0" 1.0 _returnvalue 0.0 0 0 0))
    (:1
      (Audio|PlaySoundatLocation "/Game/Final/Sound/Character_sounds/grunt_6.grunt_6" _returnvalue_2 "0, 0, 0" 1.0 _returnvalue 0.0 0 0 0))
    (:2
      (Audio|PlaySoundatLocation "/Game/Final/Sound/Character_sounds/grunt_7.grunt_7" _returnvalue_2 "0, 0, 0" 1.0 _returnvalue 0.0 0 0 0))
    (:3
      (Audio|PlaySoundatLocation "/Game/Final/Sound/Character_sounds/grunt_8.grunt_8" _returnvalue_2 "0, 0, 0" 1.0 _returnvalue 0.0 0 0 0))
    (:4
      (Audio|PlaySoundatLocation "/Game/Final/Sound/Character_sounds/cough.cough" _returnvalue_2 "0, 0, 0" 1.0 _returnvalue 0.0 0 0 0))))