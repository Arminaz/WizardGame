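; Shared camera actor that zooms by player separation, registering itself with FinalGamemode on BeginPlay.
; CameraStart caches the gamemode's player array, makes this camera every PlayerController's view target, and starts a looping UpdateCamera timer.
; UpdateCamera appends each pairwise player distance to PlayerDistances and sets spring arm length to the clamped maximum.
; PlayerDistances is never cleared here, so that maximum only grows.
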(event EventBeginPlay
  (bind _asfinal_gamemode (Utilities|Casting|CastToFinalGamemode (Game|GetGameMode)))
  (Variables|/Game/Final/Blueprints/FinalGamemode.FinalGamemode_C|SetCameraReference _asfinal_gamemode self))

(fn ConstructionScript)

(fn CameraSetup
  (bind _asfinal_gamemode (Utilities|Casting|CastToFinalGamemode (Game|GetGameMode)))
  (bind _output_get (Variables|Default|SetGamemode _asfinal_gamemode))
  (Variables|Default|SetNewVar_1 (Variables|/Game/Final/Blueprints/FinalGamemode.FinalGamemode_C|GetplayersArray _output_get))
  (bind _outactors (Actor|GetAllActorsOfClass "/Script/Engine.PlayerController"))
  (Game|Player|SetViewTargetwithBlend _outactors self 0.0 "VTBlend_Linear" 0.0 false))

(fn UpdateCamera
  (for (_array_element _array_index) (Variables|Default|GetNewVar_1)
    (for _index (range (+ _array_index 1) (- (Utilities|Array|Length (Variables|Default|GetNewVar_1)) 1))
      (Utilities|Array|Add (LocalVariables|GetplayerDistances) (Transformation|GetDistanceTo _array_element (Utilities|Array|Get(acopy) (Variables|Default|GetNewVar_1) _index)))))
  (Variables|/Script/Engine.SpringArmComponent|SetTargetArmLength (Variables|Default|GetSpringArm) (Math|Float|Clamp(Float) (.MaxValue (Math|Float|MaxOfFloatArray (LocalVariables|GetplayerDistances))) (Variables|Default|GetminSpringArmLength) (Variables|Default|GetmaxSpringArmLength))))

(fn CameraStart
  (CallFunction|CameraSetup)
  (Utilities|Time|SetTimerbyFunctionName self "updateCamera" (Variables|Default|GetcameraUpdateTime) true))