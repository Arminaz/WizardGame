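; Game mode for a local multiplayer wizard game that shows the main menu at BeginPlay and starts the match.
; StartGame gathers PlayerStarts, spawns players, then adds the game interface and starts the camera.
; SpawnPlayers matches start tags to player indices, creating a local player and possessing a new Wizard_BP for each.
; Each wizard gets per-player dynamic robe and hat materials plus its own SetWizColour call.
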(event EventBeginPlay
  (if (not (Variables|Default|GetGameRunning))
    (bind _returnvalue (UserInterface|CreateWidget "/Game/Final/Widgets/MainScreenHud.MainScreenHud_C" (Game|GetPlayerController 0)))
    (UserInterface|Viewport|AddtoViewport _returnvalue 0)))

(fn ConstructionScript
  (Actor|GetAllActorsOfClass "/Script/Engine.CameraActor"))

(fn GetPlayerStartPoints
  (bind _outactors (Actor|GetAllActorsOfClass "/Script/Engine.PlayerStart"))
  (Variables|Default|SetplayerStartArray _outactors))

(fn SpawnPlayers
  (for _index (range 0 (- (Variables|Default|GetmaxPlayerCount) 1))
    (LocalVariables|Setindex _index)
    (for _array_element (Variables|Default|GetplayerStartArray)
      (if (Utilities|Name|Equal(Name) (Variables|/Script/Engine.PlayerStart|GetPlayerStartTag _array_element) (Utilities|String|StringToName (Utilities|String|ToString(Integer) (LocalVariables|Getindex))))
        (Class|GameplayStatics|CreatePlayer (LocalVariables|Getindex))
        (bind _returnvalue (Game|SpawnActorfromClass "/Game/Final/Blueprints/Wizard_BP.Wizard_BP_C" (Transformation|GetActorTransform _array_element) "AlwaysSpawn" 0 0))
        (Variables|/Game/Final/Blueprints/Wizard_BP.Wizard_BP_C|SetplayerControllerIndex _returnvalue (LocalVariables|Getindex))
        ;[1 1 1] I don't like that I do this in the gamemode BP
        (CallFunction|SetRobeColour _returnvalue (LocalVariables|Getindex))
        (CallFunction|SetWizColour _returnvalue (LocalVariables|Getindex))
        (Pawn|Possess (Game|GetPlayerController (LocalVariables|Getindex)) _returnvalue)
        (Utilities|Array|AddUnique (Variables|Default|GetplayersArray) _returnvalue)))))

(fn SetRobeColour
  (params (WizardBP :type Wizard%20BP%20Object%20Reference) (index :type Integer))
  (bind _mesh (Variables|/Script/Engine.Character|GetMesh WizardBP))
  (bind _hat (Variables|/Game/Final/Blueprints/Wizard_BP.Wizard_BP_C|GetHat WizardBP))
  (switch int index
    (:0
      (bind _returnvalue (Rendering|Material|CreateDynamicMaterialInstance _mesh 0 "/Game/Final/Animation/Final_Character/PalleteSwaps/Player1.Player1" "None" :!class /Script/Engine.PrimitiveComponent))
      (LocalVariables|SetrobeColour _returnvalue)
      (bind _returnvalue_2 (Rendering|Material|CreateDynamicMaterialInstance _hat 1 "/Game/Final/Animation/Final_Character/PalleteSwaps/Player1_Hat.Player1_Hat" "None" :!class /Script/Engine.PrimitiveComponent))
      (LocalVariables|SetHat%20Color _returnvalue_2))
    (:1
      (bind _returnvalue_3 (Rendering|Material|CreateDynamicMaterialInstance _mesh 0 "/Game/Final/Animation/Final_Character/PalleteSwaps/Player2.Player2" "None" :!class /Script/Engine.PrimitiveComponent))
      (LocalVariables|SetrobeColour _returnvalue_3)
      (bind _returnvalue_4 (Rendering|Material|CreateDynamicMaterialInstance _hat 1 "/Game/Final/Animation/Final_Character/PalleteSwaps/Player2_Hat.Player2_Hat" "None" :!class /Script/Engine.PrimitiveComponent))
      (LocalVariables|SetHat%20Color _returnvalue_4))
    (:2
      (bind _returnvalue_5 (Rendering|Material|CreateDynamicMaterialInstance _mesh 0 "/Game/Final/Animation/Final_Character/PalleteSwaps/Player3.Player3" "None" :!class /Script/Engine.PrimitiveComponent))
      (LocalVariables|SetrobeColour _returnvalue_5)
      (bind _returnvalue_6 (Rendering|Material|CreateDynamicMaterialInstance _hat 1 "/Game/Final/Animation/Final_Character/PalleteSwaps/Player3_Hat.Player3_Hat" "None" :!class /Script/Engine.PrimitiveComponent))
      (LocalVariables|SetHat%20Color _returnvalue_6))
    (:3
      (bind _returnvalue_7 (Rendering|Material|CreateDynamicMaterialInstance _mesh 0 "/Game/Final/Animation/Final_Character/PalleteSwaps/Player4.Player4" "None" :!class /Script/Engine.PrimitiveComponent))
      (LocalVariables|SetrobeColour _returnvalue_7)
      (bind _returnvalue_8 (Rendering|Material|CreateDynamicMaterialInstance _hat 1 "/Game/Final/Animation/Final_Character/PalleteSwaps/Player4_Hat.Player4_Hat" "None" :!class /Script/Engine.PrimitiveComponent))
      (LocalVariables|SetHat%20Color _returnvalue_8)))
  (Rendering|Material|SetMaterial (Variables|/Script/Engine.Character|GetCapsuleComponent WizardBP) 0 (LocalVariables|GetrobeColour))
  (Rendering|Material|SetMaterial _hat 1 (LocalVariables|GetHat%20Color)))

(fn StartGame
  (Variables|Default|SetGameRunning true)
  (Variables|/Script/Engine.PlayerController|SetbShowMouseCursor (Game|GetPlayerController 0) false)
  (Class|WidgetBlueprintLibrary|SetFocustoGameViewport)
  (CallFunction|GetPlayerStartPoints)
  (CallFunction|SpawnPlayers)
  (bind _returnvalue (UserInterface|CreateWidget "/Game/Final/Widgets/GameInterface.GameInterface_C"))
  (UserInterface|Viewport|AddtoViewport _returnvalue 0)
  (Default|CameraStart (Variables|Default|GetCameraReference)))

(fn SetWizColour
  (params (NewParam :type Wizard%20BP%20Object%20Reference) (index :type Integer))
  (Default|SetWizColour NewParam index))