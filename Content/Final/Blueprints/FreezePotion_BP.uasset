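; Thrown freeze potion projectile that launches along the owning wizard's throw vector and bursts on first overlap, ignoring its owner by display-name comparison.
; On impact it scales the sphere collision to the area of effect and applies a status effect, with random grunts, to every overlapping wizard.
; The burst adds camera shake, a destructible bottle and freezing sound, and the actor destroys itself after a delay.
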(event OnComponentBeginOverlap(SphereCollision)
  (params (OverlappedComponent :type Primitive%20Component%20Object%20Reference) (OtherActor :type Actor%20Object%20Reference) (OtherComp :type Primitive%20Component%20Object%20Reference) (OtherBodyIndex :type Integer) (bFromSweep :type Boolean) (SweepResult :type Hit%20Result%20Structure%20%28by%20ref%29))
  (if (not (Variables|Default|Getexploded)) ; Make sure bomb is active
    (bind _aswizard_bp (Utilities|Casting|CastToWizard_BP OtherActor)
      (:then
        (if (not (Utilities|Enum|Equal(Enum) (Utilities|GetDisplayName _aswizard_bp) (Utilities|GetDisplayName (Components|GetOwner self)))) ; Check if this is my own bomb
          (Variables|Default|SethitWizard true)
          (Audio|PlaySoundatLocation "/Game/Final/Sound/Gameplay_sounds/critical_hit.critical_hit" (Transformation|GetWorldLocation (Variables|Default|GetSphereCollision)) "0, 0, 0" 0.7 1.0 0.0 0 0 0)
          (Variables|Default|Setexploded true :!label _label)
          (Transformation|SetRelativeScale3D (Variables|Default|GetSphereCollision) (Variables|Default|GetareaOfEffect))
          (CallFunction|CheckWizardDistances)
          (CallFunction|PotionExplodeEffects)
          (Collision|SetActorEnableCollision false)
          (Effects|Components|ParticleSystem|SetEmitterEnable (Variables|Default|GetThrow_Effect) "Throw" false)
          (Utilities|FlowControl|Delay 5.0)
          (Actor|DestroyActor)))
      (:CastFailed
        (goto _label)))))

(event EventBeginPlay)

(event EventEndPlay
  (params (EndPlayReason :type EEndPlayReason%20Enum :default "Destroyed")))

(fn ConstructionScript
  (bind _aswizard_bp (Utilities|Casting|CastToWizard_BP (Components|GetOwner)))
  (Game|Components|ProjectileMovement|SetVelocityinLocalSpace (Variables|Default|GetProjectileMovement) (Variables|/Game/Final/Blueprints/Wizard_BP.Wizard_BP_C|GetcurrentThrowVector _aswizard_bp)))

(fn CheckWizardDistances
  (for _array_element (Collision|GetOverlappingActors (Variables|Default|GetSphereCollision) "/Game/Final/Blueprints/Wizard_BP.Wizard_BP_C" :!class /Script/Engine.PrimitiveComponent) ; Loop over each Wizard
    (bind _aswizard_bp (Utilities|Casting|CastToWizard_BP _array_element))
    (Variables|/Game/Final/Blueprints/Wizard_BP.Wizard_BP_C|SetstatusEffect _aswizard_bp "NewEnumerator0")
    (Default|ApplyStatusEffect _aswizard_bp)
    (CallFunction|PlayHitSounds)))

(fn PlayHitSounds
  (bind _returnvalue (Math|Random|RandomFloatinRange 0.9 1.1))
  (bind _spherecollision (Variables|Default|GetSphereCollision))
  (bind _returnvalue_2 (Transformation|GetWorldLocation _spherecollision))
  ;[1 1 1] Randomized grunt noise is played when hit.
  (switch int (Math|Random|RandomInteger 5)
    (:0
      (Audio|PlaySoundatLocation "/Game/Final/Sound/Character_sounds/grunt.grunt" _returnvalue_2 "0, 0, 0" 1.0 _returnvalue 0.0 0 0 0))
    (:1
      (Audio|PlaySoundatLocation "/Game/Final/Sound/Character_sounds/grunt_2.grunt_2" _returnvalue_2 "0, 0, 0" 1.0 _returnvalue 0.0 0 0 0))
    (:2
      (Audio|PlaySoundatLocation "/Game/Final/Sound/Character_sounds/grunt_3.grunt_3" _returnvalue_2 "0, 0, 0" 1.0 _returnvalue 0.0 0 0 0))
    (:3
      (Audio|PlaySoundatLocation "/Game/Final/Sound/Character_sounds/grunt_4.grunt_4" _returnvalue_2 "0, 0, 0" 1.0 _returnvalue 0.0 0 0 0))
    (:4
      (Audio|PlaySoundatLocation "/Game/Final/Sound/Character_sounds/cough.cough" _returnvalue_2 "0, 0, 0" 1.0 _returnvalue 0.0 0 0 0))))

(fn PotionExplodeEffects
  (Camera|PlayWorldCameraShake "/Game/Final/Blueprints/CameraShake.CameraShake_C" (Transformation|GetActorLocation) 0.0 1e+10)
  (Components|DestroyComponent (Variables|Default|GetPotionBottle))
  (Game|SpawnActorfromClass "/Game/Final/Blueprints/DestructablePotion_BP.DestructablePotion_BP_C" (Transformation|GetActorTransform) "Undefined" 0 0)
  (CallFunction|PlayExplosionSound)
  (return))

(fn ApplyHapticFeedback
  (bind _asfinal_gamemode (Utilities|Casting|CastToFinalGamemode (Game|GetGameMode)))
  (for _index (range 0 (- (Variables|/Game/Final/Blueprints/FinalGamemode.FinalGamemode_C|GetmaxPlayerCount _asfinal_gamemode) 1))
    (Class|PlayerController|PlayHapticEffect (Game|GetPlayerController _index) 0 "Left" 1.0 false)))

(fn PlayExplosionSound
  (Audio|PlaySoundatLocation "/Game/Final/Sound/Gameplay_sounds/freezing_potion_effect.freezing_potion_effect" (Transformation|GetWorldLocation (Variables|Default|GetSphereCollision)) "0, 0, 0" 1.0 1.0 0.0 0 0 0))