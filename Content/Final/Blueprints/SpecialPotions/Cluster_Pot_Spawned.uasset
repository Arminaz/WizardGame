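; Spawned bomblet of the cluster potion, launched with a random upward scatter velocity and armed for overlaps after a brief delay.
; It explodes once on overlapping anything except sibling bomblets or its owner wizard, which it identifies by fragile display-name comparison.
; Exploding enlarges the sphere, runs wizard-distance and physics-impulse calls, plays effects, then destroys the actor later.
; Wizard hits play a critical sound instead of the scorch decal and explosion sound.
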(event OnComponentBeginOverlap(SphereCollision)
  (params (OverlappedComponent :type Primitive%20Component%20Object%20Reference) (OtherActor :type Actor%20Object%20Reference) (OtherComp :type Primitive%20Component%20Object%20Reference) (OtherBodyIndex :type Integer) (bFromSweep :type Boolean) (SweepResult :type Hit%20Result%20Structure%20%28by%20ref%29))
  (if (not (Variables|Default|Getexploded)) ; Make sure bomb is active
    (bind _aswizard_bp (Utilities|Casting|CastToWizard_BP OtherActor)
      (:then
        (if (not (Utilities|Enum|Equal(Enum) (Utilities|GetDisplayName _aswizard_bp) (Utilities|GetDisplayName (Components|GetOwner self)))) ; Check if this is my own bomb
          (Variables|Default|SethitWizard true)
          (Audio|PlaySoundatLocation "/Game/Final/Sound/Gameplay_sounds/critical_hit.critical_hit" (Transformation|GetWorldLocation (Variables|Default|GetSphereCollision)) "0, 0, 0" 0.7 1.0 0.0 0 0 0)
          (Variables|Default|Setexploded true :!label _label)
          (Transformation|SetRelativeScale3D (Variables|Default|GetSphereCollision) (Variables|Default|GetareaOfEffect))
          (CallFunction|CheckWizardDistances)
          (CallFunction|ApplyImpulsetoPhysicsObjects)
          (CallFunction|PotionExplodeEffects)
          (Collision|SetActorEnableCollision false)
          (Effects|Components|ParticleSystem|SetEmitterEnable (Variables|Default|GetThrow_Effect) "Throw" false)
          (Utilities|FlowControl|Delay 5.0)
          (Actor|DestroyActor)))
      (:CastFailed
        (Utilities|Casting|CastToCluster_Pot_Spawned OtherActor
          (:CastFailed
            (goto _label)))))))

(event EventBeginPlay
  (Utilities|FlowControl|Delay 0.2)
  (Collision|SetCollisionEnabled (Variables|Default|GetSphereCollision) "QueryAndPhysics"))

(event Collision|EventActorBeginOverlap
  (params (OtherActor :type Actor%20Object%20Reference)))

(event EventTick
  (params (DeltaSeconds :type Float%20%28single-precision%29)))

(event Collision|EventHit
  (params (MyComp :type Primitive%20Component%20Object%20Reference) (Other :type Actor%20Object%20Reference) (OtherComp :type Primitive%20Component%20Object%20Reference) (bSelfMoved :type Boolean) (HitLocation :type Vector :default "0, 0, 0") (HitNormal :type Vector :default "0, 0, 0") (NormalImpulse :type Vector :default "0, 0, 0") (Hit :type Hit%20Result%20Structure%20%28by%20ref%29)))

(event EventPotionExplodeEffects
  (bind _defaultsceneroot (Variables|Default|GetDefaultSceneRoot))
  (bind _returnvalue (Transformation|GetWorldLocation _defaultsceneroot))
  (Camera|PlayWorldCameraShake "/Game/Final/Blueprints/CameraShake.CameraShake_C" (Transformation|GetActorLocation) 0.0 1e+10)
  (Components|DestroyComponent (Variables|Default|GetPotionBottle))
  (Game|SpawnActorfromClass "/Game/Final/Blueprints/DestructablePotion_BP.DestructablePotion_BP_C" (Transformation|GetActorTransform) "Undefined" 0 0)
  (Effects|SpawnEmitteratLocation "/Game/Final/Particles/Explosion/Explosion_P.Explosion_P" _returnvalue)
  (if (not (Variables|Default|GethitWizard))
    (Rendering|Decal|SpawnDecalatLocation "/Game/Final/Materials/Scorch/Scorch_M.Scorch_M" "5.000000,100.000000,100.000000" (+ _returnvalue "0, 0,-10.000000") "-90.000000,0.000000,0.000000" 6e+01) ; X scale is up for some reason?
    (Audio|PlaySoundatLocation "/Game/Final/Sound/Gameplay_sounds/scatter_bomb_explosions.scatter_bomb_explosions" (Transformation|GetWorldLocation (Variables|Default|GetSphereCollision)) "0, 0, 0" 2.0 1.0 0.0 0 0 0)))

(fn ConstructionScript
  (Collision|SetCollisionEnabled (Variables|Default|GetSphereCollision) "PhysicsOnly")
  (Game|Components|ProjectileMovement|SetVelocityinLocalSpace (Variables|Default|GetProjectileMovement) (Math|Vector|MakeVector (Math|Random|RandomFloatinRange -1.5e+02 1.5e+02) (Math|Random|RandomFloatinRange -1.5e+02 1.5e+02) (Math|Random|RandomFloatinRange 2e+02 3e+02))))