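; SpecialPotionBox_BP is a cauldron pickup that gives a wizard a random special potion.
; Tick spins the actor by setting its yaw one degree past the Cauldron's current world yaw, independent of delta time.
; When a Wizard_BP hits the Cauldron, it randomly sets one of three potion types and its count, plays a pickup sound and destroys itself.
; The first hit from anything else plays an impact sound, gated by DoOnce.
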(event OnComponentHit(Cauldron)
  (params (HitComponent :type Primitive%20Component%20Object%20Reference) (OtherActor :type Actor%20Object%20Reference) (OtherComp :type Primitive%20Component%20Object%20Reference) (NormalImpulse :type Vector :default "0, 0, 0") (Hit :type Hit%20Result%20Structure%20%28by%20ref%29))
  (bind _aswizard_bp (Utilities|Casting|CastToWizard_BP OtherActor)
    (:then
      (switch int (Math|Random|RandomIntegerinRange 0 2)
        (:0
          (Variables|/Game/Final/Blueprints/Wizard_BP.Wizard_BP_C|SetspecialPotion _aswizard_bp "NewEnumerator0")
          (Variables|/Game/Final/Blueprints/Wizard_BP.Wizard_BP_C|SetnumSpecialPotions _aswizard_bp 2))
        (:1
          (Variables|/Game/Final/Blueprints/Wizard_BP.Wizard_BP_C|SetspecialPotion _aswizard_bp "NewEnumerator1")
          (Variables|/Game/Final/Blueprints/Wizard_BP.Wizard_BP_C|SetnumSpecialPotions _aswizard_bp 2))
        (:2
          (Variables|/Game/Final/Blueprints/Wizard_BP.Wizard_BP_C|SetspecialPotion _aswizard_bp "NewEnumerator2")
          (Variables|/Game/Final/Blueprints/Wizard_BP.Wizard_BP_C|SetnumSpecialPotions _aswizard_bp 1)))
      (Audio|PlaySoundatLocation "/Game/Final/Sound/Gameplay_sounds/new_potion_pickup.new_potion_pickup" (Transformation|GetActorLocation) "0, 0, 0" 1.0 1.3 0.0 0 0 0)
      (Actor|DestroyActor))
    (:CastFailed
      (Utilities|FlowControl|DoOnce false
        (:Completed
          (Audio|PlaySoundatLocation "/Game/Final/Sound/Environment/cauldron_impact.cauldron_impact" (Transformation|GetActorLocation) "0, 0, 0" 1.0 1.0 0.0 0 0 0))))))

(event EventBeginPlay)

(event Collision|EventActorBeginOverlap
  (params (OtherActor :type Actor%20Object%20Reference)))

(event EventTick
  (params (DeltaSeconds :type Float%20%28single-precision%29))
  (Transformation|SetActorRelativeRotation (Math|Rotator|MakeRotator 0.0 0.0 (+ (.yaw (Transformation|GetWorldRotation (Variables|Default|GetCauldron))) 1.0))))

(fn ConstructionScript)