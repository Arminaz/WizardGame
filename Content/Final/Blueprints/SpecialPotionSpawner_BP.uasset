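; Spawner actor that keeps dropping special potion boxes at random points around itself once the game is running.
; It polls the FinalGamemode's GameRunning flag every second, then loops without rechecking it.
; Each cycle waits a random delay, spawns an effects actor at a random XY offset, then spawns SpecialPotionBox_BP there five seconds later.
; The random CurrentSpawn box pick does not affect the drop point, and the cauldron torque is disabled.
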(event EventBeginPlay
  (bind _returnvalue (Math|Random|RandomFloatinRange -2e+02 2e+02))
  (bind _asfinal_gamemode (Utilities|Casting|CastToFinalGamemode (Game|GetGameMode)))
  (Utilities|FlowControl|RetriggerableDelay 1.0 :!label _label)
  (if (Variables|/Game/Final/Blueprints/FinalGamemode.FinalGamemode_C|GetGameRunning _asfinal_gamemode)
    (Utilities|FlowControl|RetriggerableDelay (Math|Random|RandomFloatinRange 1.0 5.0) :!label _label_2)
    (switch int (Math|Random|RandomIntegerinRange 0 3)
      (:Default
        (Variables|Default|SetCurrentSpawn (Variables|Default|GetBox3)))
      (:0
        (Variables|Default|SetCurrentSpawn (Variables|Default|GetBox)))
      (:1
        (Variables|Default|SetCurrentSpawn (Variables|Default|GetBox1)))
      (:2
        (Variables|Default|SetCurrentSpawn (Variables|Default|GetBox2))))
    (bind _output_get (Variables|Default|SetNext_Drop_Point (Math|Conversions|ToTransform(Vector) (+ (Transformation|GetActorLocation) (Math|Vector|MakeVector _returnvalue _returnvalue 0.0)))))
    (Game|SpawnActorfromClass "/Game/Final/Blueprints/Potion_Spawner_Effects_Actor.Potion_Spawner_Effects_Actor_C" _output_get "Undefined" 0 0)
    (Utilities|FlowControl|Delay 5.0)
    (bind _returnvalue_2 (Game|SpawnActorfromClass "/Game/Final/Blueprints/SpecialPotionBox_BP.SpecialPotionBox_BP_C" (Variables|Default|GetNext_Drop_Point) "AlwaysSpawn" 0 0))
    (goto _label_2)
    (else
      (goto _label))))

(event Collision|EventActorBeginOverlap
  (params (OtherActor :type Actor%20Object%20Reference)))

(event EventTick
  (params (DeltaSeconds :type Float%20%28single-precision%29)))

(fn ConstructionScript)