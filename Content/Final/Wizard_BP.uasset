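; Wizard player character that moves on axis input and aims potion throws with a second pair of throw axes.
; Throw axes drive DrawThrowArrow, which builds ThrowVector from stick direction, a lift scaled by deflection and current velocity, then previews it as a debug arrow.
; ThrowBomb spawns an owned Potion_BP above the capsule but is not called in this graph, and ApplyBombImpulse is an empty stub.
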(event EventBeginPlay)

(event Collision|EventActorBeginOverlap
  (params (OtherActor :type Actor%20Object%20Reference)))

(event EventTick
  (params (DeltaSeconds :type Float%20%28single-precision%29)))

(event Input|AxisEvents|InputAxisRightThrowAxis
  (params (AxisValue :type Float%20%28single-precision%29))
  ;[1 1 1] Draw throw arrow
  (CallFunction|DrawThrowArrow AxisValue (stale Input|AxisEvents|InputAxisUpThrowAxis AxisValue)))

(event Input|AxisEvents|InputAxisUpThrowAxis
  (params (AxisValue :type Float%20%28single-precision%29))
  ;[1 1 1] Draw throw arrow
  (CallFunction|DrawThrowArrow (stale Input|AxisEvents|InputAxisRightThrowAxis AxisValue) AxisValue))

(event Input|AxisEvents|InputAxisUpMoveAxis
  (params (AxisValue :type Float%20%28single-precision%29))
  ;[1 1 1] Movement
  (Pawn|Input|AddMovementInput (Math|Vector|MakeVector AxisValue 0.0 0.0) 1.0 false))

(event Input|AxisEvents|InputAxisRightMoveAxis
  (params (AxisValue :type Float%20%28single-precision%29))
  ;[1 1 1] Movement
  (Pawn|Input|AddMovementInput (Math|Vector|MakeVector 0.0 AxisValue 0.0) 1.0 false))

(fn ConstructionScript)

(fn ApplyBombImpulse
  (params (NewParam :type Vector)))

(fn ThrowBomb
  (Game|SpawnActorfromClass "/Game/Prototype/Potion_BP.Potion_BP_C" (Math|Transform|MakeTransform (+ (Transformation|GetWorldLocation (Variables|Collision|GetCapsuleComponent)) "0,0.000000,100.000000")) "AlwaysSpawn" self 0))

(fn DrawThrowArrow
  (params (RightAxis :type Float%20%28single-precision%29) (UpAxis :type Float%20%28single-precision%29))
  (bind _returnvalue (Transformation|GetActorLocation))
  (bind _returnvalue_2 (+ _returnvalue "0, 0,50.000000"))
  (bind _output_get (Variables|Default|SetthrowVector (+ (* (Math|Vector|MakeVector (* UpAxis -1.0) RightAxis (/ (Math|Float|Clamp(Float) (+ (Math|Float|Absolute(Float) RightAxis) (Math|Float|Absolute(Float) UpAxis))) 4.0)) 7e+02) (Transformation|GetVelocity))))
  (Rendering|Debug|DrawDebugArrow _returnvalue_2 (+ _output_get _returnvalue_2) 2e+02 "(R=0.000000,G=0.150885,B=1.000000,A=1.000000)" 0.0 1e+01))